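; Mario-style power box that releases its HiddenItem (mushroom, star, fire flower or coins) when its Box collision is overlapped.
; Power-ups play a sound, destroy the collision, switch to a used-brick material and spawn at Target; the fire flower branch currently spawns Bp_Mushroom.
; Coin hits decrement NumberOfCoin, update MarioGameInstance and briefly show a spawned coin, disabling the box once empty.
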(event OnComponentBeginOverlap(Box)
  (params (OverlappedComponent :type Primitive%20Component%20Object%20Reference) (OtherActor :type Actor%20Object%20Reference) (OtherComp :type Primitive%20Component%20Object%20Reference) (OtherBodyIndex :type Integer) (bFromSweep :type Boolean) (SweepResult :type Hit%20Result%20Structure%20%28by%20ref%29))
  ;[1 1 1] Action when Player Hit box
  (switch Utilities|FlowControl|Switch|SwitchonPowerUps (Variables|Default|GetHiddenItem)
    (:NewEnumerator1
      (CallFunction|AddMushroom))
    (:NewEnumerator2
      (CallFunction|AddStar))
    (:NewEnumerator3
      (CallFunction|AddFireFlower))
    (:NewEnumerator4
      (CallFunction|AddCoins))))

(event Custom|DestroyBoxColision
  ;[1 1 1] Destroy box component to prevent overlap again
  (Components|DestroyComponent (Variables|Default|GetBox)))

(event Custom|AddCoins
  (bind _target (Variables|Default|Gettarget))
  (bind _returnvalue (Transformation|GetWorldTransform _target))
  ;[1 1 1] Add Coins
  (Audio|PlaySoundatLocation "/Game/Mario/Sound/smb_coin.smb_coin" (Transformation|GetActorLocation))
  (if (> (Variables|Coins|GetNumberOfCoin) 0)
    (Variables|Coins|SetNumberOfCoin (- (Variables|Coins|GetNumberOfCoin) 1))
    (Default|UpdateCoinNumber (Variables|Default|GetGI) 1)
    (bind _returnvalue_2 (Game|SpawnActorfromClass "/Game/Mario/BluePrints/Bp_Coin.Bp_Coin_C" (Math|Transform|MakeTransform (.location _returnvalue) (.rotation _returnvalue) "0.300000,0.300000,0.300000") "DontSpawnIfColliding" 0 0))
    (Variables|Default|SetcurrentCoin _returnvalue_2)
    (Utilities|FlowControl|Delay 0.2)
    (Actor|DestroyActor (Variables|Default|GetcurrentCoin))
    (if (not (> (Variables|Coins|GetNumberOfCoin) 0))
      (CallFunction|DestroyBoxColision)
      (Rendering|Material|SetMaterial (Variables|Default|GetCoin_Box) 0 "/Game/Mario/Material/GoldBox/Brick3.Brick3"))))

(event Custom|AddMushroom
  (bind _target (Variables|Default|Gettarget))
  (bind _returnvalue (Transformation|GetWorldTransform _target))
  ;[1 1 1] Add Mushroom
  (Audio|PlaySoundatLocation "/Game/Mario/Sound/smb_powerup_appears.smb_powerup_appears" (Transformation|GetActorLocation))
  (CallFunction|DestroyBoxColision)
  (Rendering|Material|SetMaterial (Variables|Default|GetCoin_Box) 0 "/Game/Mario/Material/GoldBox/Brick3.Brick3")
  (Game|SpawnActorfromClass "/Game/Mario/BluePrints/Bp_Mushroom.Bp_Mushroom_C" (Math|Transform|MakeTransform (.location _returnvalue) (.rotation _returnvalue) "0.200000,0.200000,0.200000") "DontSpawnIfColliding" 0 0))

(event Custom|AddStar
  ;[1 1 1] Add Star
  (Audio|PlaySoundatLocation "/Game/Mario/Sound/smb_powerup_appears.smb_powerup_appears" (Transformation|GetActorLocation))
  (CallFunction|DestroyBoxColision)
  (Rendering|Material|SetMaterial (Variables|Default|GetCoin_Box) 0 "/Game/Mario/Material/GoldBox/Brick3.Brick3")
  (Game|SpawnActorfromClass "/Game/Mario/BluePrints/Bp_Star.Bp_Star_C" (Math|Transform|MakeTransform (.location (Transformation|GetWorldTransform (Variables|Default|Gettarget))) "0, 0, 0" "0.100000,0.100000,0.100000") "DontSpawnIfColliding" 0 0))

(event Custom|AddFireFlower
  (bind _target (Variables|Default|Gettarget))
  (bind _returnvalue (Transformation|GetWorldTransform _target))
  ;[1 1 1] Add FierFlower
  (Audio|PlaySoundatLocation "/Game/Mario/Sound/smb_powerup_appears.smb_powerup_appears" (Transformation|GetActorLocation))
  (CallFunction|DestroyBoxColision)
  (Rendering|Material|SetMaterial (Variables|Default|GetCoin_Box) 0 "/Game/Mario/Material/GoldBox/Brick3.Brick3")
  (Game|SpawnActorfromClass "/Game/Mario/BluePrints/Bp_Mushroom.Bp_Mushroom_C" (Math|Transform|MakeTransform (.location _returnvalue) (.rotation _returnvalue) "0.200000,0.200000,0.200000") "DontSpawnIfColliding" 0 0))

(event EventBeginPlay
  ;[1 1 1] Get GameInstance
  (bind _asmario_game_instance (Utilities|Casting|CastToMarioGameInstance (Game|GetGameInstance)))
  (Variables|Default|SetGI _asmario_game_instance))

(fn ConstructionScript)