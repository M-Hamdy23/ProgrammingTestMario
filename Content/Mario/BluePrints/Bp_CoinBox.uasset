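; Mario-style coin box that pays out a limited number of coins when its Box trigger is overlapped.
; Each overlap plays the coin sound; while coins remain, it decrements the count and runs a timeline that shakes the box.
; That timeline's update restarts a second one that moves the coin, which resets to its stored location after a delay.
; An overlap with none left destroys the trigger and switches the box to rusted metal.
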(event OnComponentBeginOverlap(Box)
  (params (OverlappedComponent :type Primitive%20Component%20Object%20Reference) (OtherActor :type Actor%20Object%20Reference) (OtherComp :type Primitive%20Component%20Object%20Reference) (OtherBodyIndex :type Integer) (bFromSweep :type Boolean) (SweepResult :type Hit%20Result%20Structure%20%28by%20ref%29))
  (Audio|PlaySoundatLocation "/Game/Mario/Sound/smb_coin.smb_coin" (Transformation|GetActorLocation))
  (if (> (Variables|Default|GetNumberOfCoin) 0)
    (Variables|Default|SetNumberOfCoin (- (Variables|Default|GetNumberOfCoin) 1))
    (bind _locationtrack (Timeline|Timeline_ShackCoinBox Play)
      (:Update
        (Transformation|AddRelativeLocation (Variables|Default|GetCoin_Box) _locationtrack false false)
        (bind _locationtrack_2 (Timeline|Timeline_1 PlayFromStart)
          (:Update
            (Transformation|AddRelativeLocation (Variables|Default|GetCoin) _locationtrack_2 false false))))
      (:Finished
        (Utilities|FlowControl|Delay 1.0)
        (Transformation|SetRelativeLocation (Variables|Default|GetCoin) (Variables|Default|GetCoinLocation) false false)))
    (else
      (CallFunction|DestroyBoxColision)
      (Rendering|Material|SetMaterial (Variables|Default|GetCoin_Box) 0 "/Game/Mario/Material/GoldBox/M_Metal_Rust.M_Metal_Rust"))))

(event Custom|DestroyBoxColision
  (Components|DestroyComponent (Variables|Default|GetBox)))

(fn ConstructionScript)