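; Mario-style mushroom power-up that slides along the Y axis and powers up the side-scroller character.
; The physics Cube gets its velocity at BeginPlay, then every tick once a short downward trace finds a StaticMeshActor and latches IsGround.
; Overlapping a pipe teleport actor flips the Speed sign to reverse direction.
; The Box overlap calls MushroomPower on the character and destroys the mushroom.
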(event OnComponentBeginOverlap(Cube)
  (params (OverlappedComponent :type Primitive%20Component%20Object%20Reference) (OtherActor :type Actor%20Object%20Reference) (OtherComp :type Primitive%20Component%20Object%20Reference) (OtherBodyIndex :type Integer) (bFromSweep :type Boolean) (SweepResult :type Hit%20Result%20Structure%20%28by%20ref%29)))

(event OnComponentBeginOverlap(Box)
  (params (OverlappedComponent :type Primitive%20Component%20Object%20Reference) (OtherActor :type Actor%20Object%20Reference) (OtherComp :type Primitive%20Component%20Object%20Reference) (OtherBodyIndex :type Integer) (bFromSweep :type Boolean) (SweepResult :type Hit%20Result%20Structure%20%28by%20ref%29))
  (bind _asside_scroller_character (Utilities|Casting|CastToSideScrollerCharacter OtherActor))
  (Default|MushroomPower _asside_scroller_character)
  (Actor|DestroyActor))

(event Collision|EventActorBeginOverlap
  (params (OtherActor :type Actor%20Object%20Reference))
  (Utilities|Casting|CastToBp_PipeTeleport OtherActor)
  (Variables|Default|SetSpeed (* (Variables|Default|GetSpeed) -1.0))
  (Development|PrintString (Utilities|String|ToString(Float) (* (Variables|Default|GetSpeed) -1.0))))

(event EventTick
  (params (DeltaSeconds :type Float%20%28single-precision%29))
  (bind _cube (Variables|Default|GetCube))
  (bind _returnvalue (Transformation|GetWorldLocation _cube))
  (bind (_x _y _z) (Math|Vector|BreakVector _returnvalue))
  (if (Variables|Default|GetisGround?)
    (Physics|SetPhysicsLinearVelocity (Variables|Default|GetCube) (Math|Vector|MakeVector 0.0 (Variables|Default|GetSpeed) 0.0) false "None")
    (else
      (bind _outhit (Collision|LineTraceByChannel _returnvalue (Math|Vector|MakeVector _x _y (- _z 25.0)) "TraceTypeQuery1" false 0 "ForDuration"))
      (Utilities|Casting|CastToStaticMeshActor (.HitActor (Collision|BreakHitResult _outhit)))
      (Variables|Default|SetisGround? true))))

(event EventBeginPlay
  (Physics|SetPhysicsLinearVelocity (Variables|Default|GetCube) (Math|Vector|MakeVector 0.0 (Variables|Default|GetSpeed) 0.0) false "None"))

(fn ConstructionScript)