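; Breakable Mario-style brick actor that shatters when anything overlaps its Box trigger.
; The overlap applies damage to the ShapeCubeDM destructible at the box location with an upward direction and no impulse strength, and plays the break sound.
; After a short delay it disables Plane collision and sets the destructible to physics-only collision.
; The actor destroys itself two seconds later.
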(event OnComponentBeginOverlap(Box)
  (params (OverlappedComponent :type Primitive%20Component%20Object%20Reference) (OtherActor :type Actor%20Object%20Reference) (OtherComp :type Primitive%20Component%20Object%20Reference) (OtherBodyIndex :type Integer) (bFromSweep :type Boolean) (SweepResult :type Hit%20Result%20Structure%20%28by%20ref%29))
  (Class|DestructibleComponent|ApplyDamage (Variables|Default|GetShape_Cube_DM) 1.0 (Transformation|GetWorldLocation (Variables|Default|GetBox)) (Math|Vector|MakeVector 0.0 0.0 1.0) 0.0)
  (Audio|PlaySoundatLocation "/Game/Mario/Sound/smb_breakblock.smb_breakblock" (Transformation|GetActorLocation))
  (Utilities|FlowControl|Delay 0.2)
  (Collision|SetCollisionEnabled (Variables|Default|GetPlane) "NoCollision")
  (Collision|SetCollisionEnabled (Variables|Default|GetShape_Cube_DM) "PhysicsOnly")
  (Utilities|FlowControl|Delay 2.0)
  (Actor|DestroyActor))

(fn ConstructionScript)