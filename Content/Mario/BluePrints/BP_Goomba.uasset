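; Goomba enemy for a Mario-style side-scroller that patrols along the Y axis as a physics-driven cube.
; It gets a velocity once at BeginPlay and reverses its Y velocity when it overlaps a pipe teleport actor.
; A player overlapping Box stomps it, playing a sound and destroying it.
; A player overlapping DeathTrigger gets EnemyHitYou, with the IsHit flag and a Delay acting as a hit cooldown.
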(event OnComponentBeginOverlap(DeathTrigger)
  (params (OverlappedComponent :type Primitive%20Component%20Object%20Reference) (OtherActor :type Actor%20Object%20Reference) (OtherComp :type Primitive%20Component%20Object%20Reference) (OtherBodyIndex :type Integer) (bFromSweep :type Boolean) (SweepResult :type Hit%20Result%20Structure%20%28by%20ref%29))
  (bind _asside_scroller_character (Utilities|Casting|CastToSideScrollerCharacter OtherActor))
  (if (Variables|Default|GetisHit)
    (Default|EnemyHitYou _asside_scroller_character)
    (Variables|Default|SetisHit false)
    (Utilities|FlowControl|Delay 2.0)
    (Variables|Default|SetisHit true)))

(event OnComponentBeginOverlap(Box)
  (params (OverlappedComponent :type Primitive%20Component%20Object%20Reference) (OtherActor :type Actor%20Object%20Reference) (OtherComp :type Primitive%20Component%20Object%20Reference) (OtherBodyIndex :type Integer) (bFromSweep :type Boolean) (SweepResult :type Hit%20Result%20Structure%20%28by%20ref%29))
  (Utilities|Casting|CastToSideScrollerCharacter OtherActor)
  (Audio|PlaySound2D "/Game/Mario/Sound/smb_stomp.smb_stomp")
  (Actor|DestroyActor))

(event EventBeginPlay
  (Physics|SetPhysicsLinearVelocity (Variables|Default|GetCube) "0.000000,100.000000, 0" false "None"))

(event Collision|EventActorBeginOverlap
  (params (OtherActor :type Actor%20Object%20Reference))
  (Utilities|Casting|CastToBp_PipeTeleport OtherActor)
  (bind _returnvalue (Physics|GetPhysicsLinearVelocity (Variables|Default|GetCube) "None"))
  (Physics|SetPhysicsLinearVelocity (Variables|Default|GetCube) (Math|Vector|MakeVector (.X (Math|Vector|BreakVector _returnvalue)) (* (.Y (Math|Vector|BreakVector _returnvalue)) -1.0) (.Z (Math|Vector|BreakVector _returnvalue))) false "None"))

(fn ConstructionScript)