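; Mario-style warp pipe actor that teleports the player to a target point and houses a moving hazard flower.
; A box overlap enables input, so pressing Down briefly drops the tube's collision, then teleports the player; leaving the actor disables input.
; A timeline drives the flower's vertical physics velocity.
; Touching the flower hurts the side-scroller character, or destroys the flower if the character has star power.
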(event OnComponentBeginOverlap(Box)
  (params (OverlappedComponent :type Primitive%20Component%20Object%20Reference) (OtherActor :type Actor%20Object%20Reference) (OtherComp :type Primitive%20Component%20Object%20Reference) (OtherBodyIndex :type Integer) (bFromSweep :type Boolean) (SweepResult :type Hit%20Result%20Structure%20%28by%20ref%29))
  (Input|EnableInput (Game|GetPlayerController 0)))

(event OnComponentBeginOverlap(FloowerCollision)
  (params (OverlappedComponent :type Primitive%20Component%20Object%20Reference) (OtherActor :type Actor%20Object%20Reference) (OtherComp :type Primitive%20Component%20Object%20Reference) (OtherBodyIndex :type Integer) (bFromSweep :type Boolean) (SweepResult :type Hit%20Result%20Structure%20%28by%20ref%29))
  (bind _flower (Variables|Default|GetFlower))
  (bind _asside_scroller_character (Utilities|Casting|CastToSideScrollerCharacter OtherActor))
  (if (Variables|/Game/SideScrollerBP/Blueprints/SideScrollerCharacter.SideScrollerCharacter_C|GetHasStarPower _asside_scroller_character)
    (Variables|Default|SetFlowerDie true)
    (Utilities|IsValid _flower
      (:Is%20Valid
        (Components|DestroyComponent _flower)))
    (else
      (Default|EnemyHitYou _asside_scroller_character)
      (Development|PrintString "Hello"))))

(event Collision|EventActorEndOverlap
  (params (OtherActor :type Actor%20Object%20Reference))
  (Input|DisableInput (Game|GetPlayerController 0)))

(event EventBeginPlay
  (bind _newtrack_1 (Timeline|Timeline_0 Play)
    (:Update
      (if (Variables|Default|GetFlowerDie)
        (Timeline|Timeline_0 Stop)
        (else
          (Physics|SetPhysicsLinearVelocity (Variables|Default|GetFlower) (Math|Vector|MakeVector 0.0 0.0 (* (.z _newtrack_1) 3.5)) false "None"))))))

(event Input|ActionEvents|InputActionDown
  (params (Key :type Key%20Structure))
  (:Pressed
    (Utilities|IsValid (Variables|Default|GetTargetPoint)
      (:Is%20Valid
        (Collision|SetCollisionEnabled (Variables|Default|GetShape_Tube) "NoCollision")
        (Utilities|FlowControl|Delay 0.5)
        (Collision|SetCollisionEnabled (Variables|Default|GetShape_Tube) "QueryAndPhysics")
        (Transformation|Teleport (Game|GetPlayerCharacter 0) (Transformation|GetWorldLocation (Variables|/Script/Engine.TargetPoint|GetSpriteComponent (Variables|Default|GetTargetPoint))) "0, 0, 0")))))

(fn ConstructionScript)